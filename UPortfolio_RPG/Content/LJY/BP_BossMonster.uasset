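; Boss monster Blueprint that launches an attack at a random spot within a fixed area.
; A Delay on Tick repeatedly calls AttackRange, which spawns a MonsterAttack1 actor, stores its location, starts a looping timer and immediately destroys the actor.
; The spawneffect event spawns a Niagara effect at the stored location.
; Dragon animation and spawn timeline logic is present but disconnected.
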(event `self.ReceiveBeginPlay`)

(event `self.ReceiveTick`
  (params (DeltaSeconds :type "Float (single-precision)"))
  (`KismetSystemLibrary.Delay` 3.0)
  (`self.AttackRange`))

(event `Key|X`
  (params (Key :type "Key Structure")))

(event `spawn effect`
  (`NiagaraFunctionLibrary.SpawnSystemAtLocation` "/Game/KTP_Effect/Particles/Bottom/Bottom05-03.Bottom05-03" (`self.AttackRangeLocation`)))

(fn `AttackRange`
  (bind _returnvalue (`|SpawnActorFromClass` "/Game/LJY/MonsterAttack1.MonsterAttack1_C" (`KismetMathLibrary.MakeTransform` (`KismetMathLibrary.MakeVector` (`KismetMathLibrary.RandomFloatInRange` -1040.0 340.0) (`KismetMathLibrary.RandomFloatInRange` -570.0 -30.0))) "Undefined" "MultiplyWithRoot" null null))
  (set `self.AttackRangeLocation` (`self.K2_GetActorLocation` _returnvalue))
  (`KismetSystemLibrary.K2_SetTimerDelegate` (`|CreateDelegate` :!event `spawn effect`) 1.0 true)
  (`self.K2_DestroyActor` _returnvalue))

(fn `UserConstructionScript`)