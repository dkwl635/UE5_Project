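; BP_NPCManager is a manager that handles entering and leaving NPC interaction.
; The interaction input toggles on the Interactior flag, blending the player's view to the current NPC or back to the stored pawn.
; InteractiorNPC or LeaveNPC runs after the blend delay.
; Debug leftovers include "Hello" prints, an S key that saves the player inventory, and an unconnected drop-item spawn chain.
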(event `EnhancedInput|/Game/KJW/Input/IA_Interaction`
  (params (ActionValue :type Boolean) (ElapsedSeconds :type "Float (double-precision)") (TriggeredSeconds :type "Float (double-precision)") (InputAction :type "InputAction Object Reference" :default "/Game/KJW/Input/IA_Interaction.IA_Interaction"))
  (:`Started`
    (`KismetSystemLibrary.PrintString` "Hello")
    (if (`self.bInteractior`)
      (`self.EndInteractiorNPC`)
      (else
        (`self.StartInteractiorNPC`)))))

(event `self.ReceiveStartInteractiorNPC`
  (bind _returnvalue (`GameplayStatics.GetPlayerController` 0))
  (bind _blend_time (`self.Blend Time`))
  (set `self.PlayerCharacter` (`Controller.K2_GetPawn` _returnvalue))
  (`PlayerController.SetViewTargetWithBlend` _returnvalue (`self.CurrentNPC`) _blend_time "VTBlend_Linear" 0.0 false)
  (`KismetSystemLibrary.Delay` _blend_time)
  (`self.InteractiorNPC`))

(event `self.ReceiveEndInteractiorNPC`
  (bind _blend_time (`self.Blend Time`))
  (`PlayerController.SetViewTargetWithBlend` (`GameplayStatics.GetPlayerController` 0) (`self.PlayerCharacter`) _blend_time "VTBlend_Linear" 0.0 false)
  (`KismetSystemLibrary.Delay` _blend_time)
  (`self.LeaveNPC`))

(event `Key|S`
  (params (Key :type "Key Structure"))
  (:`Pressed`
    (`PlayerInventorySubsystem.Save` (subsystem `PlayerInventorySubsystem`))
    (`KismetSystemLibrary.PrintString` "Hello")))

(fn `UserConstructionScript`)