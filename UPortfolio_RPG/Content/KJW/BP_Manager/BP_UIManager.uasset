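; UI manager Blueprint that routes player input to the RPG interface.
; One second after BeginPlay it sizes PlayerUI to the viewport size divided by viewport scale.
; Enhanced Input actions hide the top UI on Back and call GetRPGUIToggle for the inventory and equipment screens.
; The hide and toggle logic is defined outside these graphs.
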(event `self.ReceiveBeginPlay`
  (`KismetSystemLibrary.Delay` 1.0)
  (`RPGMainUserWidget.SetViewSize` (`self.PlayerUI`) (/ (`WidgetLayoutLibrary.GetViewportSize`) (`WidgetLayoutLibrary.GetViewportScale`))))

(event `EnhancedInput|/Game/KJW/Input/IA_UIBack`
  (params (ActionValue :type Boolean) (ElapsedSeconds :type "Float (double-precision)") (TriggeredSeconds :type "Float (double-precision)") (InputAction :type "InputAction Object Reference" :default "/Game/KJW/Input/IA_UIBack.IA_UIBack"))
  (:`Started`
    (`self.TopHideUI`)))

(event `EnhancedInput|/Game/KJW/Input/IA_Inventory`
  (params (ActionValue :type Boolean) (ElapsedSeconds :type "Float (double-precision)") (TriggeredSeconds :type "Float (double-precision)") (InputAction :type "InputAction Object Reference" :default "/Game/KJW/Input/IA_Inventory.IA_Inventory"))
  (:`Triggered`
    (`self.GetRPGUIToggle` "INVENTORY")))

(event `EnhancedInput|/Game/KJW/Input/IA_Equipment`
  (params (ActionValue :type Boolean) (ElapsedSeconds :type "Float (double-precision)") (TriggeredSeconds :type "Float (double-precision)") (InputAction :type "InputAction Object Reference" :default "/Game/KJW/Input/IA_Equipment.IA_Equipment"))
  (:`Triggered`
    (`self.GetRPGUIToggle` "EQUIPMENT")))

(fn `UserConstructionScript`)