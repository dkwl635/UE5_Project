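; NPC interaction manager that toggles the view between the player's pawn and the current NPC on the interaction input.
; BeginPlay registers the interaction mapping context, and each press starts or ends the interaction based on the Interactior flag.
; Starting stores the pawn and blends the view target to CurrentNPC, while ending blends back.
; Each path waits out the blend time before calling InteractiorNPC or LeaveNPC.
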(event `self.ReceiveBeginPlay`
  (bind _returnvalue (`GameplayStatics.GetPlayerController` 0))
  (`/Engine/EditorBlueprintResources/StandardMacros.IsValid` _returnvalue
    (:`Is Valid`
      (`EnhancedInputSubsystemInterface.AddMappingContext` (pcsubsystem `EnhancedInputLocalPlayerSubsystem` _returnvalue) "/Game/KJW/Input/IMC_Interaction.IMC_Interaction" 0 (struct)))))

(event `EnhancedInput|/Game/KJW/Input/IA_Interaction`
  (params (ActionValue :type Boolean) (ElapsedSeconds :type "Float (double-precision)") (TriggeredSeconds :type "Float (double-precision)") (InputAction :type "InputAction Object Reference" :default "/Game/KJW/Input/IA_Interaction.IA_Interaction"))
  (:`Started`
    (if (`self.bInteractior`)
      (`self.EndInteractiorNPC`)
      (else
        (`self.StartInteractiorNPC`)))))

(event `self.ReceiveStartInteractiorNPC`
  (bind _returnvalue (`GameplayStatics.GetPlayerController` 0))
  (bind _blend_time (`self.Blend Time`))
  (set `self.PlayerCharacter` (`Controller.K2_GetPawn` _returnvalue))
  (`PlayerController.SetViewTargetWithBlend` _returnvalue (`self.CurrentNPC`) _blend_time "VTBlend_Linear" 0.0 false)
  (`KismetSystemLibrary.Delay` _blend_time)
  (`self.InteractiorNPC`))

(event `self.ReceiveEndInteractiorNPC`
  (bind _blend_time (`self.Blend Time`))
  (`PlayerController.SetViewTargetWithBlend` (`GameplayStatics.GetPlayerController` 0) (`self.PlayerCharacter`) _blend_time "VTBlend_Linear" 0.0 false)
  (`KismetSystemLibrary.Delay` _blend_time)
  (`self.LeaveNPC`))

(fn `UserConstructionScript`)